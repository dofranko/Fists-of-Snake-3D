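; BP_FoSGameState is a game state Blueprint that keeps an elapsed match timer in minutes and seconds.
; StartTimer sets a flag that lets Tick count, using a one-second Delay to pace increments and roll seconds over into minutes.
; GetTimer returns the time as a minutes:seconds string, zero-padding seconds below ten.
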(event Custom|Start%20Timer
  (Variables|Default|SetIsStarted true))

(event EventBeginPlay)

(event EventTick
  (params (DeltaSeconds :type Float%20%28single-precision%29))
  (if (Variables|Default|GetIsStarted)
    (Utilities|FlowControl|Delay 1.0)
    (Variables|Default|SetSeconds (+ (Variables|Default|GetSeconds) 1))
    (if (> (Variables|Default|GetSeconds) 59)
      (Variables|Default|SetMinutes (+ (Variables|Default|GetMinutes) 1))
      (Variables|Default|SetSeconds 0))))

(fn ConstructionScript)

(fn GetTimer
  (bind _seconds (Variables|Default|GetSeconds))
  (if (< _seconds 10)
    (LocalVariables|SetSecondsTrue (Utilities|String|Append "0" (Utilities|String|ToString(Integer) _seconds)))
    (else
      (LocalVariables|SetSecondsTrue (Utilities|String|ToString(Integer) _seconds))))
  (return (Utilities|String|Append (Utilities|String|Append (Utilities|String|ToString(Integer) (Variables|Default|GetMinutes)) ":") (LocalVariables|GetSecondsTrue))))